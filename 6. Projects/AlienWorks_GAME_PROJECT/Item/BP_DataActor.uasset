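; BP_DataActor is an actor that tests reading stats from a DataTable.
; On BeginPlay it looks up the row Entry1 in the Example table.
; When the row is found, it stores the Level, Hp and Attack fields in its variables and prints each to the screen.
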(event `self.ReceiveBeginPlay`
  (bind _returnvalue (`|GetDataTableRow` "/Game/PCH_PRIVATE/ExcelData/Example.Example" "Entry1")
    (:`then`
      (bind (_level _hp _attack) (break `/Game/PCH_PRIVATE/ExcelData/FData` _returnvalue))
      (set `self.Level` _level)
      (set `self.Hp` _hp)
      (set `self.Attack` _attack)
      (`KismetSystemLibrary.PrintString` (`KismetStringLibrary.Conv_DoubleToString` (`self.Level`)))
      (`KismetSystemLibrary.PrintString` (`KismetStringLibrary.Conv_DoubleToString` (`self.Hp`)))
      (`KismetSystemLibrary.PrintString` (`KismetStringLibrary.Conv_DoubleToString` (`self.Attack`))))))

(fn `UserConstructionScript`)