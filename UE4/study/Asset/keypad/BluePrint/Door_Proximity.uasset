(event `self.Box.OnComponentBeginOverlap`
  (params (OverlappedComponent :type "PrimitiveComponent Object Reference") (OtherActor :type "Actor Object Reference") (OtherComp :type "PrimitiveComponent Object Reference") (OtherBodyIndex :type Integer) (bFromSweep :type Boolean) (SweepResult :type "HitResult Structure (by ref)"))
  (bind _asthird_person_character (cast `/Game/ThirdPersonBP/Blueprints/ThirdPersonCharacter` OtherActor))
  (for (_array_element _array_index) (`/Game/ThirdPersonBP/Blueprints/ThirdPersonCharacter.KeyArm` _asthird_person_character)
    (if (and _array_element (== _array_index (`self.keyArm value`)))
      (`self.EnableInput` null)
      (bind (_direction _doorsliding) (`Timeline|Door Animation`)
        (:`Update`
          (`SceneComponent.K2_SetRelativeLocation` (`self.DoorMesh`) _doorsliding false false)))
      (else
        (`KismetSystemLibrary.PrintString` "You Need a Arm!")))))

(fn `UserConstructionScript`)